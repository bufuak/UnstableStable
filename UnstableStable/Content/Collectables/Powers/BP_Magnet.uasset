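; BP_Magnet is a magnet power-up collectable that greatly enlarges the pickup reach of BP_HorseShoe.
; On any actor overlap it destroys itself, then, if that actor is a BP_HorseShoe, scales up its SphereCollision.
; A trailing Delay leads to nothing, so the scale is never restored here.
; A disconnected older version toggles a timed MagnetPickedUp flag on ThirdPersonGameMode and never runs.
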(event EventBeginPlay)

(event Collision|EventActorBeginOverlap
  (params (OtherActor :type Actor%20Object%20Reference))
  (Actor|DestroyActor)
  (bind _asbp_horse_shoe (Utilities|Casting|CastToBP_HorseShoe OtherActor))
  (Transformation|SetWorldScale3D (Variables|/Game/Collectables/Coins/BP_HorseShoe.BP_HorseShoe_C|GetSphereCollision _asbp_horse_shoe) "100.000000,100.000000,100.000000")
  (Utilities|FlowControl|Delay 5.0))

(event EventTick
  (params (DeltaSeconds :type Float%20%28single-precision%29)))

(fn ConstructionScript)
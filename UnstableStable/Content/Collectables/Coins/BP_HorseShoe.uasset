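; BP_HorseShoe is a collectable pickup that adds to the player's coin count.
; Overlap by the ThirdPersonCharacter plays the CoinGetsCloser timeline, which sweeps the actor from its sphere collision's current location toward the player.
; On the timeline's update, a DoOnce increments Coins on ThirdPersonGameMode, then after a short delay plays a sound, prints the total and destroys the actor.
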(event Collision|EventActorBeginOverlap
  (params (OtherActor :type Actor%20Object%20Reference))
  (Utilities|Casting|CastToThirdPersonCharacter OtherActor)
  (bind _coingetscloser (Timeline|CoinGetsCloser Play)
    (:Update
      (Transformation|SetActorLocation (Math|Vector|Lerp(Vector) (Transformation|GetWorldLocation (Variables|Default|GetSphereCollision)) (Transformation|GetActorLocation (Game|GetPlayerCharacter 0)) _coingetscloser) true false)
      (bind _asthird_person_game_mode (Utilities|Casting|CastToThirdPersonGameMode (Game|GetGameMode)))
      (bind _output_get (Variables|Default|SetAs%20Third%20Person%20Game%20Mode _asthird_person_game_mode))
      (Utilities|FlowControl|DoOnce false
        (:Completed
          (bind _result (Math|Integer|IncrementInt (Variables|/Game/ThirdPersonBP/Blueprints/ThirdPersonGameMode.ThirdPersonGameMode_C|GetCoins _output_get))
            (:%20%20
              (bind _output_get_2 (Variables|/Game/ThirdPersonBP/Blueprints/ThirdPersonGameMode.ThirdPersonGameMode_C|SetCoins (Variables|Default|GetAs%20Third%20Person%20Game%20Mode) _result))
              (Utilities|FlowControl|Delay 0.2)
              (Audio|PlaySound2D "/Game/Collectables/Coins/mixkit-game-treasure-coin-2038.mixkit-game-treasure-coin-2038" 1.0 1.0 0.0 0 0)
              (Development|PrintString (Utilities|String|ToString(Integer) _output_get_2))
              (Actor|DestroyActor))))))))

(fn ConstructionScript)
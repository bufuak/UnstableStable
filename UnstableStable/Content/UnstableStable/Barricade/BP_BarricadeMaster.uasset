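; BP_BarricadeMaster is a barricade obstacle actor that breaks away when the player character runs into it.
; The construction script randomly assigns one of two obstacle meshes to its static mesh component.
; A component hit from the player character destroys only that mesh component, leaving the actor itself in the level.
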(event OnComponentHit(SM_Obstacle_3)
  (params (HitComponent :type Primitive%20Component%20Object%20Reference) (OtherActor :type Actor%20Object%20Reference) (OtherComp :type Primitive%20Component%20Object%20Reference) (NormalImpulse :type Vector :default "0, 0, 0") (Hit :type Hit%20Result%20Structure%20%28by%20ref%29))
  (if (== OtherActor (Game|GetPlayerCharacter 0))
    (Components|DestroyComponent (Variables|Default|GetSM_Obstacle_3))))

(event EventBeginPlay)

(event Collision|EventActorBeginOverlap
  (params (OtherActor :type Actor%20Object%20Reference)))

(event EventTick
  (params (DeltaSeconds :type Float%20%28single-precision%29)))

(fn ConstructionScript
  (Components|StaticMesh|SetStaticMesh (Variables|Default|GetSM_Obstacle_3) (Utilities|Select :Index (Math|Random|RandomIntegerinRange 0 1) :Option%200 "/Game/UnstableStable/Meshes/SM_Obb.SM_Obb" :Option%201 "/Game/UnstableStable/Meshes/SM_Obstacle_3.SM_Obstacle_3")))
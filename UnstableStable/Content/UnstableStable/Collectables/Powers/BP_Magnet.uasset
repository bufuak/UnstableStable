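; BP_Magnet is a collectable power-up that grants ThirdPersonCharacter a timed magnet state.
; On overlap it sets MagnetPickedUp on the character and hides itself, then after a fixed delay clears the flag and destroys itself.
; The actor only toggles that flag, and the graph also holds debug prints and unconnected leftover nodes.
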(event Collision|EventActorBeginOverlap
  (params (OtherActor :type Actor%20Object%20Reference))
  (bind _asthird_person_character (Utilities|Casting|CastToThirdPersonCharacter OtherActor))
  (bind _output_get (Variables|Default|SetAs%20Third%20Person%20Character _asthird_person_character))
  (Variables|/Game/ThirdPersonBP/Blueprints/ThirdPersonCharacter.ThirdPersonCharacter_C|SetMagnetPickedUp? _output_get true)
  (Development|PrintString "Magnet Active")
  (Rendering|SetActorHiddenInGame true)
  (Utilities|FlowControl|Delay 1e+01)
  (Variables|/Game/ThirdPersonBP/Blueprints/ThirdPersonCharacter.ThirdPersonCharacter_C|SetMagnetPickedUp? (Variables|Default|GetAs%20Third%20Person%20Character) false)
  (Development|PrintString "Hello")
  (Actor|DestroyActor))

(fn ConstructionScript)
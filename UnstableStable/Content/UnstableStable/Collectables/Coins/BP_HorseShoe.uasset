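; BP_HorseShoe is a collectable horseshoe that counts as one coin when the farmer collects it.
; Box overlap handles normal pickup, while the larger-purpose MagnetCollision pulls it in only if the farmer holds a magnet, clearing InRange to block the normal path.
; Both paths use timelines to lerp from the spawn location to the player.
; A DoOnce on timeline update credits StableGameMode, then plays a sound and destroys the actor after a delay.
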(event OnComponentBeginOverlap(MagnetCollision)
  (params (OverlappedComponent :type Primitive%20Component%20Object%20Reference) (OtherActor :type Actor%20Object%20Reference) (OtherComp :type Primitive%20Component%20Object%20Reference) (OtherBodyIndex :type Integer) (bFromSweep :type Boolean) (SweepResult :type Hit%20Result%20Structure%20%28by%20ref%29))
  ;[1 1 1] Collecting Horseshoe with Magnet
  (bind _asbp_farmer (Utilities|Casting|CastToBP_Farmer OtherActor))
  (if (Variables|/Game/ThirdPersonBP/Blueprints/ThirdPersonCharacter.ThirdPersonCharacter_C|GetMagnetPickedUp? _asbp_farmer)
    (Variables|Default|SetInRange false)
    (bind _coingetscloser (Timeline|Timeline_0 PlayFromStart)
      (:Update
        (Transformation|SetActorLocation (Math|Vector|Lerp(Vector) (Variables|Default|GetActorLocation) (Transformation|GetActorLocation (Game|GetPlayerCharacter 0)) _coingetscloser) true false)
        (Utilities|FlowControl|DoOnce false
          (:Completed
            (Default|GetCoin (Variables|Default|GetAs%20Stable%20Game%20Mode) 1)
            (Utilities|FlowControl|Delay 1.0)
            (Audio|PlaySound2D "/Game/UnstableStable/Collectables/Coins/mixkit-game-treasure-coin-2038.mixkit-game-treasure-coin-2038" 1.0 1.0 0.0 0 0)
            (Actor|DestroyActor)))))))

(event OnComponentBeginOverlap(Box)
  (params (OverlappedComponent :type Primitive%20Component%20Object%20Reference) (OtherActor :type Actor%20Object%20Reference) (OtherComp :type Primitive%20Component%20Object%20Reference) (OtherBodyIndex :type Integer) (bFromSweep :type Boolean) (SweepResult :type Hit%20Result%20Structure%20%28by%20ref%29))
  ;[1 1 1] Collecting Horseshoe without Magnet
  (if (Variables|Default|GetInRange)
    (bind _asbp_farmer (Utilities|Casting|CastToBP_Farmer OtherActor))
    (Variables|Default|SetAs%20BP%20Farmer _asbp_farmer)
    (bind _coingetscloser (Timeline|CoinGetsCloser Play)
      (:Update
        (Transformation|SetActorLocation (Math|Vector|Lerp(Vector) (Variables|Default|GetActorLocation) (Transformation|GetActorLocation (Game|Player|GetPlayerPawn 0)) _coingetscloser) true false)
        (Utilities|FlowControl|DoOnce false
          (:Completed
            (Default|GetCoin (Variables|Default|GetAs%20Stable%20Game%20Mode) 1)
            (Utilities|FlowControl|Delay 0.2)
            (Audio|PlaySound2D "/Game/UnstableStable/Collectables/Coins/mixkit-game-treasure-coin-2038.mixkit-game-treasure-coin-2038" 1.0 1.0 0.0 0 0)
            (Actor|DestroyActor)))))))

(event EventBeginPlay
  (bind _asstable_game_mode (Utilities|Casting|CastToStableGameMode (Game|GetGameMode)))
  (Variables|Default|SetAs%20Stable%20Game%20Mode _asstable_game_mode)
  (Variables|Default|SetActorLocation (Transformation|GetActorLocation)))

(fn ConstructionScript)
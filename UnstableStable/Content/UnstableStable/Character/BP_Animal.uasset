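; BP_Animal is an animal character whose Boom event turns the player back into a farmer.
; Boom spawns the NS_BackFarmer effect and a BP_Farmer at the player pawn's transform, copying AxisState across.
; The player controller then possesses the farmer, StableGameMode's IsFarmer is set, and the animal destroys itself.
; A delayed cleanup of the effect component is sequenced after that self-destruction.
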(event EventBeginPlay
  (|CallParentFunction) ; This node is disabled and will not be called.\nDrag off pins to build functionality.
)

(event Collision|EventActorBeginOverlap
  (params (OtherActor :type Actor%20Object%20Reference))
  (|CallParentFunction OtherActor) ; This node is disabled and will not be called.\nDrag off pins to build functionality.
)

(event EventTick
  (params (DeltaSeconds :type Float%20%28single-precision%29))
  (|CallParentFunction DeltaSeconds) ; This node is disabled and will not be called.\nDrag off pins to build functionality.
)

(event EventBoom
  (bind _output_get (Variables|Default|SetTransform (Transformation|GetActorTransform (Game|Player|GetPlayerPawn 0))))
  (bind _returnvalue (Niagara|SpawnSystematLocation "/Game/Effect/NS_BackFarmer.NS_BackFarmer" (.location _output_get) (.rotation _output_get)))
  (Utilities|FlowControl|Sequence
    (:then_0
      (bind _returnvalue_2 (Game|SpawnActorfromClass "/Game/UnstableStable/Character/BP_Farmer.BP_Farmer_C" (Variables|Default|GetTransform) "Undefined" 0 0))
      (Variables|/Game/UnstableStable/Character/BP_Farmer.BP_Farmer_C|SetAxisState _returnvalue_2 (Variables|Default|GetAxisState))
      (Pawn|UnPossess (Game|GetPlayerController 0))
      (Pawn|Possess (Game|GetPlayerController 0) _returnvalue_2)
      (bind _asstable_game_mode (Utilities|Casting|CastToStableGameMode (Game|GetGameMode)))
      (Variables|/Game/UnstableStable/StableGameMode.StableGameMode_C|SetIsFarmer _asstable_game_mode true)
      (Actor|DestroyActor))
    (:then_1
      (Utilities|FlowControl|Delay 1.0)
      (Components|DestroyComponent _returnvalue))))

(fn ConstructionScript
  (|CallParentFunction))
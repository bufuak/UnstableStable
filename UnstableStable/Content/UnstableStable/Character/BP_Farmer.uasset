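; BP_Farmer is an auto-running player character that switches between four fixed lanes and can transform into farm animals.
; Tick drives forward movement, Left/Right teleport between lanes by AxisState, and Up/Down set walk speed.
; K opens the UnstableTransformation widget.
; The UnstableTransformation event replaces the pawn with the chosen animal amid a Niagara poof, passing on lane, possession and the game mode's max speed.
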(event Custom|UnstableTransformation
  (params (AnimalEnum :type AnimalEnum%20Enum :default "NewEnumerator0"))
  ;[1 1 1] Comment
  (bind _output_get (Variables|Default|SetTransform (Transformation|GetActorTransform (Game|Player|GetPlayerPawn 0))))
  (bind _returnvalue (Niagara|SpawnSystematLocation "/Game/Effect/NS_Poof.NS_Poof" (.location _output_get) (.rotation _output_get)))
  (Utilities|FlowControl|Sequence
    (:then_0
      (Pawn|UnPossess (Game|GetPlayerController 0))
      (Actor|DestroyActor)
      (bind _returnvalue_2 (Game|SpawnActorfromClass (Utilities|Select :Index AnimalEnum :NewEnumerator0 "/Game/UnstableStable/Character/BP_Chicken.BP_Chicken_C" :NewEnumerator1 "/Game/UnstableStable/Character/BP_Cow.BP_Cow_C" :NewEnumerator2 "/Game/UnstableStable/Character/BP_Goat.BP_Goat_C" :NewEnumerator4 "/Game/UnstableStable/Character/BP_Pig.BP_Pig_C" :NewEnumerator5 "/Game/UnstableStable/Character/BP_Sheep.BP_Sheep_C") (Variables|Default|GetTransform) "Undefined" 0 0))
      (bind _asbp_farmer (Utilities|Casting|CastToBP_Farmer _returnvalue_2))
      (Variables|BP_Farmer_C|SetAxisState _asbp_farmer (Variables|Default|GetAxisState))
      (Transformation|Teleport (.location (Variables|Default|GetTransform)) (.rotation (Variables|Default|GetTransform)))
      (bind _aspawn (Utilities|Casting|CastToPawn _returnvalue_2))
      (Pawn|Possess (Game|GetPlayerController 0) _aspawn)
      (Variables|/Script/Engine.CharacterMovementComponent|SetMaxWalkSpeed (Variables|/Script/Engine.Character|GetCharacterMovement (Game|GetPlayerCharacter 0)) (Variables|/Game/UnstableStable/StableGameMode.StableGameMode_C|GetNewMaxSpeed (Variables|Default|GetAs%20Stable%20Game%20Mode))))
    (:then_1
      (Utilities|FlowControl|Delay 1.0)
      (Components|DestroyComponent _returnvalue))))

(event EventBeginPlay
  (Variables|Default|SetAxisState 2)
  (bind _asstable_game_mode (Utilities|Casting|CastToStableGameMode (Game|GetGameMode)))
  (Variables|Default|SetAs%20Stable%20Game%20Mode _asstable_game_mode))

(event Collision|EventActorBeginOverlap
  (params (OtherActor :type Actor%20Object%20Reference)))

(event EventTick
  (params (DeltaSeconds :type Float%20%28single-precision%29))
  (Pawn|Input|AddMovementInput (Transformation|GetActorForwardVector) (* DeltaSeconds 3e+02) false)
  (Variables|Default|SetSpeed (Math|Vector|VectorLength (Transformation|GetVelocity))))

(event Input|ActionEvents|InputActionRight
  (params (Key :type Key%20Structure :default "None"))
  (bind _returnvalue (Transformation|GetActorLocation))
  (:Pressed
    (if (!= (Variables|Default|GetAxisState) 3)
      (Math|Integer|IncrementInt (Variables|Default|GetAxisState)
        (:%20%20
          (Transformation|Teleport (Math|Vector|MakeVector (.x _returnvalue) (Utilities|Select :Index (Variables|Default|GetAxisState) :Option%200 -1.5e+02 :Option%201 -5e+01 :Option%202 5e+01 :Option%203 1.5e+02) (.z _returnvalue)) (Transformation|GetActorRotation)))))))

(event Input|ActionEvents|InputActionLeft
  (params (Key :type Key%20Structure :default "None"))
  (bind _returnvalue (Transformation|GetActorLocation))
  (:Pressed
    (if (!= (Variables|Default|GetAxisState) 0)
      (Math|Integer|DecrementInt (Variables|Default|GetAxisState)
        (:%20%20
          (Transformation|Teleport (Math|Vector|MakeVector (.x _returnvalue) (Utilities|Select :Index (Variables|Default|GetAxisState) :Option%200 -1.5e+02 :Option%201 -5e+01 :Option%202 5e+01 :Option%203 1.5e+02) (.z _returnvalue)) (Transformation|GetActorRotation)))))))

(event Input|AxisEvents|InputAxisMoveRight
  (params (AxisValue :type Float%20%28single-precision%29)))

(event Input|AxisEvents|InputAxisLookUp
  (params (AxisValue :type Float%20%28single-precision%29)))

(event Input|AxisEvents|InputAxisTurn
  (params (AxisValue :type Float%20%28single-precision%29)))

(event Input|KeyboardEvents|Down
  (params (Key :type Key%20Structure :default "None"))
  (:Pressed
    (Variables|/Script/Engine.CharacterMovementComponent|SetMaxWalkSpeed (Variables|Character|GetCharacterMovement) 301.0)))

(event Input|KeyboardEvents|K
  (params (Key :type Key%20Structure :default "None"))
  (:Released
    (bind _returnvalue (UserInterface|CreateWidget "/Game/UnstableStable/UI/UnstableTransformation.UnstableTransformation_C"))
    (UserInterface|Viewport|AddtoViewport _returnvalue 0)))

(event Input|KeyboardEvents|Up
  (params (Key :type Key%20Structure :default "None"))
  (:Pressed
    (Variables|/Script/Engine.CharacterMovementComponent|SetMaxWalkSpeed (Variables|Character|GetCharacterMovement) 1.2e+03)))

(fn ConstructionScript
  (|CallParentFunction))